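; RPG player character Blueprint, currently holding only debug test logic for sword attack animations.
; Four debug key presses each play one montage of the sword combo on the character mesh and print a test message if it is interrupted.
; Unconnected leftover nodes check the anim instance's jump start, loop and land flags with debug prints, but never run.
; BeginPlay, overlap and the construction script are empty.
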(event EventBeginPlay)

(event Collision|EventActorBeginOverlap
  (params (OtherActor :type Actor%20Object%20Reference)))

(event Input|KeyboardEvents|DebugKey2
  (params (Key :type Key%20Structure :default "None") (ActionValue :type Input%20Action%20Value%20Structure))
  (:Pressed
    (Animation|Montage|PlayMontage (Variables|Character|GetMesh) "/Game/RPG/Character/Player/Mannequin/Animations/Montage/LightAttack/AM_Sword_Attack_Combo_01_01_Anim_Montage.AM_Sword_Attack_Combo_01_01_Anim_Montage"
      (:OnInterrupted
        (Development|PrintString "Hello")))))

(event Input|KeyboardEvents|DebugKey3
  (params (Key :type Key%20Structure :default "None") (ActionValue :type Input%20Action%20Value%20Structure))
  (:Pressed
    (Animation|Montage|PlayMontage (Variables|Character|GetMesh) "/Game/RPG/Character/Player/Mannequin/Animations/Montage/LightAttack/AM_Sword_Attack_Combo_01_02_Anim_Montage.AM_Sword_Attack_Combo_01_02_Anim_Montage"
      (:OnInterrupted
        (Development|PrintString "Hello")))))

(event Input|KeyboardEvents|DebugKey4
  (params (Key :type Key%20Structure :default "None") (ActionValue :type Input%20Action%20Value%20Structure))
  (:Pressed
    (Animation|Montage|PlayMontage (Variables|Character|GetMesh) "/Game/RPG/Character/Player/Mannequin/Animations/Montage/LightAttack/AM_Sword_Attack_Combo_01_03_Anim_Montage.AM_Sword_Attack_Combo_01_03_Anim_Montage"
      (:OnInterrupted
        (Development|PrintString "Hello")))))

(event Input|KeyboardEvents|DebugKey5
  (params (Key :type Key%20Structure :default "None") (ActionValue :type Input%20Action%20Value%20Structure))
  (:Pressed
    (Animation|Montage|PlayMontage (Variables|Character|GetMesh) "/Game/RPG/Character/Player/Mannequin/Animations/Montage/LightAttack/AM_Sword_Attack_Combo_01_04_Anim_Montage.AM_Sword_Attack_Combo_01_04_Anim_Montage"
      (:OnInterrupted
        (Development|PrintString "Hello")))))

(fn ConstructionScript)