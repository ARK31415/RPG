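; Gameplay ability for the player's sword light attack, built as a montage combo, though its main chain has no triggering event and never runs as wired.
; That chain plays the montage mapped to the attack count in ComboMontages, then advances the count or wraps it after the last.
; When the montage completes, blends out or is stopped, the ability ends and starts a short timer that resets the combo.
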(event Custom|ResetCount
  (Variables|Default|SetAttackcount 1)
  (Development|PrintString "ResetCount")
  (Development|PrintString (Utilities|String|ToString(Integer) (Variables|Default|GetAttackcount))))

(event Ability|EventOnEndAbility
  (params (bWasCancelled :type Boolean)))