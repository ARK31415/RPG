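; RPG player controller Blueprint that sets up the game's UI when possession occurs and offers a debug enemy spawn.
; On possess it creates the primary game layout widget, registers it with the RPG UI manager subsystem, then pushes the HUD as a soft widget onto the Frontend stack.
; A debug key acquires a Gruntling Guardian from the enemy pool subsystem near the world origin and prints its name.
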(event EventBeginPlay)

(event EventTick
  (params (DeltaSeconds :type Float%20%28single-precision%29)))

(event EventPossess
  (params (PossessedPawn :type Pawn%20Object%20Reference))
  (bind _returnvalue (UserInterface|CreateWidget "/Game/RPG/UI/Widgets/WBP_CUW_RPGPrimaryGameLayout.WBP_CUW_RPGPrimaryGameLayout_C" self))
  (UserInterface|Viewport|AddtoViewport _returnvalue 0)
  (Class|RPGUIManagerSubsystem|RegisterWidgetLayoutBase (Subsystems|GetRPGUIManagerSubsystem) _returnvalue)
  (|PushSoftWidget self "/Game/RPG/UI/Widgets/WBP_RPGHUDWidget.WBP_RPGHUDWidget_C" "(TagName=\"RPGCommonUI.WidgetStack.Frontend\")" true))

(event Input|KeyboardEvents|DebugKey0
  (params (Key :type Key%20Structure :default "None") (ActionValue :type Input%20Action%20Value%20Structure))
  (:Pressed
    (bind _returnvalue (Class|RPGEnemyPoolSubsystem|AcquireEnemy (Subsystems|GetRPGEnemyPoolSubsystem) "/Game/RPG/Character/Enemy/Gruntling/Guardian/BP_Gruntling_Guardian.BP_Gruntling_Guardian_C" (Math|Transform|MakeTransform "0.000000,0.000000,10.000000")))
    (Development|PrintString (Utilities|GetDisplayName _returnvalue))))

(fn ConstructionScript)